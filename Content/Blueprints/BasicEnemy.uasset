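; BasicEnemy is an enemy that shows the player's current combat key prompt and explodes at body sockets as combat progresses.
; Every Tick reads BasicGameCharacter, showing CombatText as Q, E, Z or C from CurrentKeyNum only while InCombat.
; Tick also runs CombatParticles, which spawns P_Explosion_BP once per GetCombatValue stage, guarded by AlreadyBoom flags.
; The fourth stage tests for 40, breaking the 1-2-3 sequence.
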(event Custom|CombatParticles
  (bind _asbasic_game_character (Utilities|Casting|CastToBasicGameCharacter (Game|Player|GetPlayerPawn 0)))
  (bind _returnvalue (Class|BasicGameCharacter|GetCombatValue _asbasic_game_character))
  (if (== _returnvalue 1.0)
    (if (not (Variables|Default|GetAlreadyBoom1))
      (Game|SpawnActorfromClass "/Game/Blueprints/P_Explosion_BP.P_Explosion_BP_C" (Math|Conversions|ToTransform(Vector) (Transformation|GetSocketLocation (Variables|Character|GetMesh) "upperarm_l")) "Undefined" 0 0)
      (Variables|Default|SetAlreadyBoom1 true))
    (elif (== _returnvalue 2.0)
      (if (not (Variables|Default|GetAlreadyBoom2))
        (Game|SpawnActorfromClass "/Game/Blueprints/P_Explosion_BP.P_Explosion_BP_C" (Math|Conversions|ToTransform(Vector) (Transformation|GetSocketLocation (Variables|Character|GetMesh) "upperarm_r")) "Undefined" 0 0)
        (Variables|Default|SetAlreadyBoom2 true))
      (elif (== _returnvalue 3.0)
        (if (not (Variables|Default|GetAlreadyBoom3))
          (Game|SpawnActorfromClass "/Game/Blueprints/P_Explosion_BP.P_Explosion_BP_C" (Math|Conversions|ToTransform(Vector) (Transformation|GetSocketLocation (Variables|Character|GetMesh) "pelvis")) "Undefined" 0 0)
          (Variables|Default|SetAlreadyBoom3 true))
        (elif (== _returnvalue 4e+01)
          (if (not (Variables|Default|GetAlreadyBoom4))
            (Game|SpawnActorfromClass "/Game/Blueprints/P_Explosion_BP.P_Explosion_BP_C" (Math|Conversions|ToTransform(Vector) (Transformation|GetSocketLocation (Variables|Character|GetMesh) "spine_03")) "Undefined" 0 0)
            (Variables|Default|SetAlreadyBoom4 true)))))))

(event EventBeginPlay)

(event EventTick
  (params (DeltaSeconds :type Float%20%28single-precision%29))
  (bind _combattext (Variables|Default|GetCombatText))
  (bind _combattext_2 (Variables|Default|GetCombatText))
  (CallFunction|CombatParticles)
  (bind _asbasic_game_character (Utilities|Casting|CastToBasicGameCharacter (Game|Player|GetPlayerPawn 0)))
  (if (Variables|/Script/BasicGame.BasicGameCharacter|GetInCombat _asbasic_game_character)
    (Rendering|SetVisibility _combattext true false)
    (if (== (Variables|/Script/BasicGame.BasicGameCharacter|GetCurrentKeyNum _asbasic_game_character) 1)
      (bind _output_get (Variables|Default|SetText "Q"))
      (Rendering|Components|TextRender|SetText _combattext_2 _output_get)
      (elif (== (Variables|/Script/BasicGame.BasicGameCharacter|GetCurrentKeyNum _asbasic_game_character) 2)
        (bind _output_get_2 (Variables|Default|SetText "E"))
        (Rendering|Components|TextRender|SetText _combattext_2 _output_get_2)
        (elif (== (Variables|/Script/BasicGame.BasicGameCharacter|GetCurrentKeyNum _asbasic_game_character) 3)
          (bind _output_get_3 (Variables|Default|SetText "Z"))
          (Rendering|Components|TextRender|SetText _combattext_2 _output_get_3)
          (elif (== (Variables|/Script/BasicGame.BasicGameCharacter|GetCurrentKeyNum _asbasic_game_character) 4)
            (bind _output_get_4 (Variables|Default|SetText "C"))
            (Rendering|Components|TextRender|SetText _combattext_2 _output_get_4)))))
    (else
      (Rendering|SetVisibility _combattext false false))))

(fn ConstructionScript)